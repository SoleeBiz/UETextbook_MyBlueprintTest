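; BP_TestActor is a scratch actor for practicing basic Blueprint scripting, with no active gameplay behavior.
; Its event graph holds three disconnected experiments: a loop incrementing and printing a number, a sum printed in color, and a range branch printing Korean two-digit messages.
; The first two use a simple custom Add function.
; BeginPlay and the construction script are empty, so none of these experiments run.
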(event `self.ReceiveBeginPlay`)

(fn `Add`
  (params (Num1 :type Integer) (Num2 :type Integer))
  (returns (Result :type Integer))
  (return (+ Num1 Num2)))

(fn `UserConstructionScript`)